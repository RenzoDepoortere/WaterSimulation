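; BP_MovingActor is an actor that moves continuously along a horizontal circle around its starting location.
; BeginPlay stores the actor's location as StartPos, the circle's center.
; Each Tick sets an absolute position from degree-based cosine and sine of game time times MovementSpeed, scaled by CircleRadius, without sweep.
; MovementSpeed therefore acts as degrees per second, and the actor's rotation is left untouched.
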(event `self.ReceiveBeginPlay`
  (set `self.StartPos` (`self.K2_GetActorLocation`)))

(event `self.ReceiveTick`
  (params (DeltaSeconds :type "Float (single-precision)"))
  (bind _circleradius (`self.CircleRadius`))
  (bind _returnvalue (* (`KismetSystemLibrary.GetGameTimeInSeconds`) (`self.MovementSpeed`)))
  (`self.K2_SetActorLocation` (+ (`self.StartPos`) (`KismetMathLibrary.MakeVector` (* (`KismetMathLibrary.DegCos` _returnvalue) _circleradius) (* _circleradius (`KismetMathLibrary.DegSin` _returnvalue))))))

(fn `UserConstructionScript`)