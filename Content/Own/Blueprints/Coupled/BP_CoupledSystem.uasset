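; BP_CoupledSystem is an actor wrapping a Niagara system, apparently a FLIP simulation coupled to a moving actor.
; Two custom events cache the actor's location as FLIP height and moving-actor start point.
; Disconnected logic would spawn BP_MovingActor and feed grid center (following it at fixed height, or at this actor) and movement delta to Niagara.
; BeginPlay, Tick and the construction script are empty, so none of that logic runs.
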(event `SetFLIPHeight`
  (bind (_returnvalue_x _returnvalue_y _returnvalue_z) (`KismetMathLibrary.BreakVector` (`self.K2_GetActorLocation`)))
  ;[1 1 1] Locations
  (set `self.FLIP_Height` _returnvalue_z))

(event `SetMovingStartLocation`
  ;[1 1 1] Locations
  (set `self.MovingActorStartLocation` (`self.K2_GetActorLocation`)))

(event `self.ReceiveBeginPlay`
  ;[1 1 1] Spawn moving actor
)

(event `self.ReceiveTick`
  (params (DeltaSeconds :type "Float (single-precision)")))

(fn `UserConstructionScript`)